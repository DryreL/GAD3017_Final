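; BP_Train is a train actor that rides the spline of a referenced track, optionally starting on BeginPlay.
; The TrainBrokenBrakes timeline, with play rate set by Duration, drives location and rotation by distance along the spline and saves its progress as the start offset.
; The SlowTheTrain input lengthens Duration and restarts movement from that offset.
; The timeline update also watches for Duration changes, re-running the setup and then stopping the timeline.
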(event `self.ReceiveTick`
  (params (DeltaSeconds :type "Float (single-precision)")))

(event `self.ReceiveBeginPlay`
  ;[1 1 1] Check Train Available To Move
  (if (`self.StartWithMovement`)
    (`self.MoveTrain`)))

(event `MoveTrain`
  (bind _duration (`self.Duration`))
  ;[1 1 1] Move along Spline
  (`TimelineComponent.SetPlayRate` (`self.TrainBrokenBrakes`) (/ 1.0 _duration) :!label _label)
  (set `self.InitialDuration` _duration)
  (`TimelineComponent.SetNewTime` (`self.TrainBrokenBrakes`) (`self.TrainStartOffset`))
  (bind (_direction _alpha) (`Timeline|TrainBrokenBrakes` :`NewTime` 0.0 :!label _label_2)
    (:`Update`
      (bind _output_get (set `self.Alpha` _alpha))
      (set `self.TrainStartOffset` _output_get)
      (bind _returnvalue (`KismetMathLibrary.Lerp` 0.0 (`SplineComponent.GetSplineLength` (`/Game/Bluprint/BP_MovementTrack.Spline` (`self.TrackRef`))) _output_get))
      (`self.K2_SetActorLocationAndRotation` (`SplineComponent.GetLocationAtDistanceAlongSpline` (`/Game/Bluprint/BP_MovementTrack.Spline` (`self.TrackRef`)) _returnvalue "World") (`SplineComponent.GetRotationAtDistanceAlongSpline` (`/Game/Bluprint/BP_MovementTrack.Spline` (`self.TrackRef`)) _returnvalue "World"))
      (if (not (== (`self.InitialDuration`) (`self.Duration`)))
        (`|ExecutionSequence`
          (:`then_0`
            (set `self.InitialDuration` (`self.Duration`))
            (goto _label))
          (:`then_1`
            (goto _label_2 :!via `Stop`)))))))

(event `InputAction|SlowTheTrain`
  (params (Key :type "Key Structure"))
  ;[1 1 1] Move along Spline
  (:`Pressed`
    (bind _output_get (set `self.Duration` (* (`self.Duration`) 1.1)))
    (`self.MoveTrain`)
    (`KismetSystemLibrary.PrintString` (`KismetStringLibrary.Concat_StrStr` "Duration: " (`KismetStringLibrary.Conv_DoubleToString` _output_get) "   IDuration" (`KismetStringLibrary.Conv_DoubleToString` (`self.InitialDuration`)) "   Offset:" (`KismetStringLibrary.Conv_DoubleToString` (`self.TrainStartOffset`))))))

(fn `UserConstructionScript`)