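; Spider-web shot projectile: an impulse-launched physics sphere trailing a Niagara beam that sticks on first impact.
; Tick stretches the beam to the sphere until a hit freezes it and plays a timeline-driven hit effect.
; Hits check WebTarget tags and overwrite the target's tags, but TagChecker's train-slowdown call is unwired.
; A stop effect fades the web after a miss or timeout, and a looping timer destroys the actor.
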(event `StopEffect`
  (`/Engine/EditorBlueprintResources/StandardMacros.DoOnce` false :!label _label
    (:`Completed`
      (bind (_direction _stopeffect) (`Timeline|StopEffect_T`)
        (:`Update`
          (`FXSystemComponent.SetFloatParameter` (`self.Web`) "User.Stop" _stopeffect))))))

(event `self.ReceiveBeginPlay`
  (`|ExecutionSequence`
    (:`then_0`
      (`KismetSystemLibrary.Delay` 5.0)
      (`self.StopEffect`)
      (set `self.IsReadyToDestroy` true))
    (:`then_1`
      (`PrimitiveComponent.AddImpulse` (`self.ProjectileStickySphere`) (* (`self.GetActorForwardVector`) (* (`self.SplurgeSpeed`) 1000.0)) "None" false)
      (`KismetSystemLibrary.Delay` 1.0)
      (if (not (`self.ProjectileHit`))
        (goto _label)))
    (:`then_2`
      (`KismetSystemLibrary.K2_SetTimer` null "DestroyObject" 2.0 true))))

(event `DestroyObject`
  (if (`self.IsReadyToDestroy`)
    (`self.K2_DestroyActor`)))

(event `self.ReceiveTick`
  (params (DeltaSeconds :type "Float (single-precision)"))
  (if (not (`self.ProjectileHit`))
    (`FXSystemComponent.SetVectorParameter` (`self.Web`) "User.BeamEnd" (`SceneComponent.K2_GetComponentLocation` (`self.ProjectileStickySphere`)))
    (`FXSystemComponent.SetFloatParameter` (`self.Web`) "User.Distance" (`KismetMathLibrary.Vector_Distance` (`SceneComponent.K2_GetComponentLocation` (`self.ProjectileStickySphere`)) (`SceneComponent.K2_GetComponentLocation` (`self.Sphere`))))))

(event `self.ProjectileStickySphere.OnComponentHit`
  (params (HitComponent :type "PrimitiveComponent Object Reference") (OtherActor :type "Actor Object Reference") (OtherComp :type "PrimitiveComponent Object Reference") (NormalImpulse :type "Vector Structure") (Hit :type "HitResult Structure (by ref)"))
  (bind (_bblockinghit _binitialoverlap _time _distance _location _impactpoint) (`GameplayStatics.BreakHitResult` Hit))
  (bind _returnvalue (`KismetMathLibrary.Normal` (- _impactpoint (`SceneComponent.K2_GetComponentLocation` (`self.Sphere`)))))
  (`/Engine/EditorBlueprintResources/StandardMacros.DoOnce` false
    (:`Completed`
      (set `self.ProjectileHit` true)
      (`PrimitiveComponent.SetSimulatePhysics` (`self.ProjectileStickySphere`) false)
      (`PrimitiveComponent.SetCollisionEnabled` (`self.ProjectileStickySphere`) "NoCollision")
      (`FXSystemComponent.SetVectorParameter` (`self.Web`) "User.BeamEnd" (- _impactpoint (* _returnvalue 40.0)))
      (`FXSystemComponent.SetVectorParameter` (`self.Web`) "User.Orientation" _returnvalue)
      (`self.CallReduceTrainSpeedEventMacroed`)
      (bind (_direction _hit) (`Timeline|Hit`)
        (:`Update`
          (`FXSystemComponent.SetFloatParameter` (`self.Web`) "User.Hit" _hit))))))

(event `CallReduceTrainSpeedEventMacroed`
  (`|ExecutionSequence`
    (:`then_0`
      (`self.TagChecker` (stale `self.ProjectileStickySphere.OnComponentHit` OtherActor) "WebTarget5" 1.02 "5"))
    (:`then_1`
      (`self.TagChecker` (stale `self.ProjectileStickySphere.OnComponentHit` OtherActor) "WebTarget10" 1.05 "10"))
    (:`then_2`
      (`self.TagChecker` (stale `self.ProjectileStickySphere.OnComponentHit` OtherActor) "WebTarget20" 1.09 "20")))
  (set `Actor.Tags` (`self.TagRemoval`) (stale `self.ProjectileStickySphere.OnComponentHit` OtherActor)))

(fn `UserConstructionScript`)