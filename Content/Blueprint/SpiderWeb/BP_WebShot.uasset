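; Spider-Man-style web shot that launches a physics sphere along its forward vector plus the train's vector, trailed by a Niagara beam.
; The first hit pins sphere and beam, except that BP_Projectile actors are destroyed instead.
; Hit actors tagged WebTarget5/10/20 are hidden, call the train's speed-reduction function and add to the pawn's score.
; Timelines animate impact and fade-out, which follows a short miss timeout or longer lifetime before timed cleanup.
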(event `StopEffect`
  (`/Engine/EditorBlueprintResources/StandardMacros.DoOnce` false :!label _label
    (:`Completed`
      (bind (_direction _stopeffect) (`Timeline|StopEffect_T`)
        (:`Update`
          (`FXSystemComponent.SetFloatParameter` (`self.Web`) "User.Stop" _stopeffect))))))

(event `self.ReceiveBeginPlay`
  (`|ExecutionSequence`
    (:`then_0`
      (`GameplayStatics.PlaySound2D` "/Game/Gokdeniz/Spider-Man_web_shoot_sound_effect.Spider-Man_web_shoot_sound_effect" 1.0 1.0 0.0 null null))
    (:`then_1`
      (`KismetSystemLibrary.Delay` 10.0)
      (`self.StopEffect`)
      (set `self.IsReadyToDestroy` true))
    (:`then_2`
      (bind _outactors (`GameplayStatics.GetAllActorsOfClass` "/Game/Blueprint/BP_Train.BP_Train_C"))
      (for _array_element _outactors
        (`PrimitiveComponent.AddImpulse` (`self.ProjectileStickySphere`) (* (+ (`/Game/Blueprint/BP_Train.TrainVector` _array_element) (`self.GetActorForwardVector`)) (* (`self.SplurgeSpeed`) 4000.0)) "None" false)
        (`KismetSystemLibrary.Delay` 3.0)
        (if (not (`self.ProjectileHit`))
          (goto _label))))
    (:`then_3`
      (`KismetSystemLibrary.K2_SetTimer` null (stale `DestroyObject` FunctionName) 2.0 true))
    (:`then_4`
      (bind _asmotion_controller_pawn (cast `/Game/VirtualRealityBP/Blueprints/MotionControllerPawn` (`GameplayStatics.GetPlayerPawn` 0)))
      (set `self.MotionControllerPawnRef` _asmotion_controller_pawn))))

(event `DestroyObject`
  (params (FunctionName :type String))
  (if (`self.IsReadyToDestroy`)
    (`self.K2_DestroyActor`)))

(event `self.ReceiveTick`
  (params (DeltaSeconds :type "Float (single-precision)"))
  (`|ExecutionSequence`
    (:`then_0`
      (if (not (`self.ProjectileHit`))
        (`FXSystemComponent.SetVectorParameter` (`self.Web`) "User.BeamEnd" (`SceneComponent.K2_GetComponentLocation` (`self.ProjectileStickySphere`)))
        (`FXSystemComponent.SetFloatParameter` (`self.Web`) "User.Distance" (`KismetMathLibrary.Vector_Distance` (`SceneComponent.K2_GetComponentLocation` (`self.ProjectileStickySphere`)) (`SceneComponent.K2_GetComponentLocation` (`self.Sphere`))))))))

(event `self.ProjectileStickySphere.OnComponentHit`
  (params (HitComponent :type "PrimitiveComponent Object Reference") (OtherActor :type "Actor Object Reference") (OtherComp :type "PrimitiveComponent Object Reference") (NormalImpulse :type "Vector Structure") (Hit :type "HitResult Structure (by ref)"))
  (bind (_bblockinghit _binitialoverlap _time _distance _location _impactpoint) (`GameplayStatics.BreakHitResult` Hit))
  (bind _returnvalue (`KismetMathLibrary.Normal` (- _impactpoint (`SceneComponent.K2_GetComponentLocation` (`self.Sphere`)))))
  (bind _asbp_projectile (cast `/Game/Gokdeniz/YeniKod/BP_Projectile` OtherActor)
    (:`then`
      (`/Game/Gokdeniz/YeniKod/BP_Projectile.Destroy_Projectile` _asbp_projectile))
    (:`CastFailed`
      (`/Engine/EditorBlueprintResources/StandardMacros.DoOnce` false
        (:`Completed`
          (set `self.ProjectileHit` true)
          (`PrimitiveComponent.SetSimulatePhysics` (`self.ProjectileStickySphere`) false)
          (`PrimitiveComponent.SetCollisionEnabled` (`self.ProjectileStickySphere`) "NoCollision")
          (`FXSystemComponent.SetVectorParameter` (`self.Web`) "User.BeamEnd" (- _impactpoint (* _returnvalue 40.0)))
          (`FXSystemComponent.SetVectorParameter` (`self.Web`) "User.Orientation" _returnvalue)
          (`self.CallReduceTrainSpeedEventMacroed`)
          (bind (_direction _hit) (`Timeline|Hit`)
            (:`Update`
              (`FXSystemComponent.SetFloatParameter` (`self.Web`) "User.Hit" _hit))))))))

(event `CallReduceTrainSpeedEventMacroed`
  (`|ExecutionSequence`
    (:`then_0`
      (`self.TagCheckerOpen` (stale `self.ProjectileStickySphere.OnComponentHit` OtherActor) "WebTarget5" 1.0002 "5" 5))
    (:`then_1`
      (`self.TagCheckerOpen` (stale `self.ProjectileStickySphere.OnComponentHit` OtherActor) "WebTarget10" 1.0005 "10" 10))
    (:`then_2`
      (`self.TagCheckerOpen` (stale `self.ProjectileStickySphere.OnComponentHit` OtherActor) "WebTarget20" 1.0009 "20" 20))))

(event `TagCheckerOpen`
  (params (Target :type "Actor Object Reference") (Tag :type Name) (InputPin :type "Float (double-precision)") (InputPin2 :type String) (B :type Integer))
  (if (`self.ActorHasTag` Target Tag)
    (`GameplayStatics.PlaySound2D` "/Game/Gokdeniz/shine-collect-sound-effect-hd.shine-collect-sound-effect-hd" 1.0 1.0 0.0 null null)
    (bind _outactors (`GameplayStatics.GetAllActorsOfClass` "/Game/Blueprint/BP_Train.BP_Train_C"))
    (for _array_element _outactors
      (`/Game/Blueprint/BP_Train.ReduceTrainSpeedFunction` _array_element InputPin InputPin2)
      (set `Actor.Tags` (`self.TagRemoval`) Target)
      (`self.SetActorHiddenInGame` Target true)
      (set `/Game/VirtualRealityBP/Blueprints/MotionControllerPawn.Score` (+ (`/Game/VirtualRealityBP/Blueprints/MotionControllerPawn.Score` (`self.MotionControllerPawnRef`)) B) (`self.MotionControllerPawnRef`))
      (set `self.BillboardRef` (`self.BillboardRef`)))))

(fn `UserConstructionScript`)