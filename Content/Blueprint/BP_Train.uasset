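; Train actor that runs along a referenced track spline, slows in steps, and stops on reaching a duration limit or overlapping a "Crash"-tagged actor.
; A timeline maps progress to spline location and rotation, with play rate set to the inverse of Duration.
; ReduceTrainSpeed stretches Duration by a compounding SpeedDrop multiplier and resumes the timeline from the saved offset.
; Three test inputs trigger slowdowns of different strengths.
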(event `self.ReceiveTick`
  (params (DeltaSeconds :type "Float (single-precision)")))

(event `self.ReceiveBeginPlay`
  ;[1 1 1] Check Train Available To Move
  (if (`self.StartWithMovement`)
    (`self.MoveTrain`)))

(event `self.EndChecker.OnComponentBeginOverlap`
  (params (OverlappedComponent :type "PrimitiveComponent Object Reference") (OtherActor :type "Actor Object Reference") (OtherComp :type "PrimitiveComponent Object Reference") (OtherBodyIndex :type Integer) (bFromSweep :type Boolean) (SweepResult :type "HitResult Structure (by ref)"))
  ;[1 1 1] Ending
  (if (`self.ActorHasTag` OtherActor "Crash")
    (`self.CrashTime`)
    (`KismetSystemLibrary.PrintString` "TrainCrash")))

(event `MoveTrain`
  (bind _duration (`self.Duration`))
  ;[1 1 1] Move along Spline
  (if (not (`self.IsStopped`))
    (`TimelineComponent.SetPlayRate` (`self.TrainBrokenBrakes`) (/ 1.0 _duration) :!label _label)
    (set `self.InitialDuration` _duration)
    (`TimelineComponent.SetNewTime` (`self.TrainBrokenBrakes`) (`self.TrainStartOffset`))
    (bind (_direction _alpha) (`Timeline|TrainBrokenBrakes` :!label _label_2)
      (:`Update`
        (bind _output_get (set `self.Alpha` _alpha))
        (set `self.TrainStartOffset` _output_get)
        (bind _returnvalue (`KismetMathLibrary.Lerp` 0.0 (`SplineComponent.GetSplineLength` (`/Game/Blueprint/BP_MovementTrack.Spline` (`self.TrackRef`))) _output_get))
        (`self.K2_SetActorLocationAndRotation` (`SplineComponent.GetLocationAtDistanceAlongSpline` (`/Game/Blueprint/BP_MovementTrack.Spline` (`self.TrackRef`)) _returnvalue "World") (`SplineComponent.GetRotationAtDistanceAlongSpline` (`/Game/Blueprint/BP_MovementTrack.Spline` (`self.TrackRef`)) _returnvalue "World"))
        (if (< (`self.Duration`) (`self.DurationToStop`))
          (if (not (== (`self.InitialDuration`) (`self.Duration`)))
            (`|ExecutionSequence`
              (:`then_0`
                (set `self.InitialDuration` (`self.Duration`))
                (goto _label))
              (:`then_1`
                (goto _label_2 :!via `Stop`))))
          (else
            (set `self.IsStopped` true :!label _label_3)
            (`KismetSystemLibrary.PrintString` "TrainStopped")
            (goto _label_2 :!via `Stop`)))))))

(event `CrashTime`
  ;[1 1 1] Move along Spline
  (goto _label_3))

(event `ReduceTrainSpeedFunction`
  (params (B :type "Float (double-precision)") (H :type String))
  ;[1 1 1] ReduceTrainSpeed Call
  (`self.ReduceTrainSpeed` B H))

(event `ReduceTrainSpeed5`
  ;[1 1 1] Reduce Train Speed OOF
)

(event `InputAction|SlowTheTrain5`
  (params (Key :type "Key Structure"))
  ;[1 1 1] ReduceTrainSpeed Call
  ;;[1 1 1] Testing
  (:`Pressed`
    (`self.ReduceTrainSpeed` 1.0002 "5")))

(event `InputAction|SlowTheTrain10`
  (params (Key :type "Key Structure"))
  ;[1 1 1] ReduceTrainSpeed Call
  ;;[1 1 1] Testing
  (:`Pressed`
    (`self.ReduceTrainSpeed` 1.005 "10")))

(event `ReduceTrainSpeed10`
  ;[1 1 1] Reduce Train Speed OOF
)

(event `InputAction|SlowTheTrain20`
  (params (Key :type "Key Structure"))
  ;[1 1 1] ReduceTrainSpeed Call
  ;;[1 1 1] Testing
  (:`Pressed`
    (`self.ReduceTrainSpeed` 1.009 "20")))

(event `ReduceTrainSpeed20`
  ;[1 1 1] Reduce Train Speed OOF
)

(fn `UserConstructionScript`)