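; BP_MovementTrack is a track actor that lays copies of a configurable mesh along a spline.
; The construction script derives spacing from the mesh's X bounds plus an offset, then fits the instance count to the spline length.
; GetLocationAtIndex supplies each instance's local position and rotation at that distance, feeding a single InstancedStaticMesh, starting one spacing in.
; The event graph has no active logic, only an unconnected BP_SplineHouses spawn.
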(event `self.ReceiveBeginPlay`)

(fn `GetLocationAtIndex`
  (params (A :type Integer))
  (returns (ReturnValue :type "Vector Structure") (Rotation :type "Rotator Structure"))
  (bind _spline (`self.Spline`))
  (bind _returnvalue (* A (`self.Spacing`)))
  (return (`SplineComponent.GetLocationAtDistanceAlongSpline` _spline _returnvalue "Local") (`SplineComponent.GetRotationAtDistanceAlongSpline` _spline _returnvalue "Local")))

(fn `UserConstructionScript`
  (bind _placed_mesh (`self.Placed Mesh`))
  (bind (_min _max) (break `Box` (`StaticMesh.GetBoundingBox` _placed_mesh)))
  (`StaticMeshComponent.SetStaticMesh` (`self.InstancedStaticMesh`) _placed_mesh)
  (bind _output_get (set `self.Spacing` (+ (.x (- _max _min)) (`self.Off Set`))))
  (bind _output_get_2 (set `self.Number Of Instances` (`KismetMathLibrary.FFloor` (/ (`SplineComponent.GetSplineLength` (`self.Spline`)) _output_get))))
  (for _index (range (+ _output_get_2 1))
    (bind (_returnvalue _rotation) (`self.GetLocationAtIndex` (+ _index 1)))
    (`InstancedStaticMeshComponent.AddInstance` (`self.InstancedStaticMesh`) (`KismetMathLibrary.MakeTransform` _returnvalue _rotation))))