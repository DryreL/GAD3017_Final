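; BP_Bullet is a projectile that damages the VR player's MotionControllerPawn when it overlaps a BP_MotionController.
; Each hit subtracts one PHealth, prints the remaining health and destroys the bullet, first calling CrashTime on the train reference if health is depleted.
; Unhit bullets self-destroy five seconds after BeginPlay.
; The BP_Train reference is assigned only in that destroy path, after DestroyActor, so nothing here sets it before a hit.
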(event `DestroyBullet`
  (`self.K2_DestroyActor` :!label _label)
  (bind _returnvalue (`GameplayStatics.GetActorOfClass` "/Game/Blueprint/BP_Train.BP_Train_C"))
  (set `self.BP_TrainRef` _returnvalue))

(event `self.ReceiveBeginPlay`
  (`KismetSystemLibrary.Delay` 5.0)
  (goto _label))

(event `self.Collision.OnComponentBeginOverlap`
  (params (OverlappedComponent :type "PrimitiveComponent Object Reference") (OtherActor :type "Actor Object Reference") (OtherComp :type "PrimitiveComponent Object Reference") (OtherBodyIndex :type Integer) (bFromSweep :type Boolean) (SweepResult :type "HitResult Structure (by ref)"))
  (cast `/Game/VirtualRealityBP/Blueprints/BP_MotionController` OtherActor)
  (bind _asmotion_controller_pawn (cast `/Game/VirtualRealityBP/Blueprints/MotionControllerPawn` (`GameplayStatics.GetPlayerPawn` 0)))
  (bind _output_get (set `/Game/VirtualRealityBP/Blueprints/MotionControllerPawn.PHealth` (- (`/Game/VirtualRealityBP/Blueprints/MotionControllerPawn.PHealth` _asmotion_controller_pawn) 1) _asmotion_controller_pawn))
  (`KismetSystemLibrary.PrintString` (`KismetStringLibrary.Concat_StrStr` (`KismetStringLibrary.Conv_IntToString` _output_get) " health left") true true (struct :`R` 1.0 :`B` 0.007701 :`A` 1.0))
  (`|ExecutionSequence`
    (:`then_0`
      (if (<= (`/Game/VirtualRealityBP/Blueprints/MotionControllerPawn.PHealth` _asmotion_controller_pawn) 0)
        (`/Game/Blueprint/BP_Train.CrashTime` (`self.BP_TrainRef`))))
    (:`then_1`
      (`self.K2_DestroyActor`))))

(fn `UserConstructionScript`)