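; BP_ThrowSystem is a turret-like actor that repeatedly spawns physics bullets in relation to the player's motion controller pawn.
; On BeginPlay it caches the pawn and starts a looping timer that calls Shoot.
; Shoot spawns a BP_Bullet at the Arrow and applies force along the pawn-to-actor vector scaled by BulletSpeed.
; It turns to face the player only after firing, and its DoOnce resets immediately.
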(event `self.ReceiveBeginPlay`
  (bind _asmotion_controller_pawn (cast `/Game/VirtualRealityBP/Blueprints/MotionControllerPawn` (`GameplayStatics.GetPlayerPawn` 0)))
  (set `self.MotionControllerPawn` _asmotion_controller_pawn)
  (`KismetSystemLibrary.K2_SetTimer` null "Shoot" 3.0 true))

(event `Shoot`
  (`/Engine/EditorBlueprintResources/StandardMacros.DoOnce` false :!label _label
    (:`Completed`
      (bind _returnvalue (`|SpawnActorFromClass` "/Game/Gokdeniz/BP_Bullet.BP_Bullet_C" (`KismetMathLibrary.MakeTransform` (`SceneComponent.K2_GetComponentLocation` (`self.Arrow`)) (`SceneComponent.K2_GetComponentRotation` (`self.Arrow`))) "Undefined" "OverrideRootScale" null null))
      (bind _bullet (`/Game/Gokdeniz/BP_Bullet.Bullet` _returnvalue))
      (`PrimitiveComponent.SetSimulatePhysics` _bullet true)
      (`PrimitiveComponent.AddForce` _bullet (* (- (`self.K2_GetActorLocation`) (`self.K2_GetActorLocation` (`self.MotionControllerPawn`))) (`self.BulletSpeed`)) "None" false)
      ;[1 0.3534 0.3833] Aim to player
      (`self.K2_SetActorRelativeRotation` (`KismetMathLibrary.FindLookAtRotation` (`self.K2_GetActorLocation`) (`self.K2_GetActorLocation` (`self.MotionControllerPawn`))))
      (goto _label :!via `Reset`))))

(fn `UserConstructionScript`)