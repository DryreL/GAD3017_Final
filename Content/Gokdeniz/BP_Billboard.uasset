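; BP_Billboard is a world billboard that displays the player's score and coin count on text render components.
; On BeginPlay it casts player pawn 0 to MotionControllerPawn, stores it, and starts a looping one-second timer that calls BillboardSystem.
; Each call reads Score and Coin from that pawn and writes labeled, formatted text to the two text renders, so updates are polled without using Tick.
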(event `self.ReceiveBeginPlay`
  (bind _asmotion_controller_pawn (cast `/Game/VirtualRealityBP/Blueprints/MotionControllerPawn` (`GameplayStatics.GetPlayerPawn` 0)))
  (set `self.As Motion Controller Pawn` _asmotion_controller_pawn)
  (`KismetSystemLibrary.K2_SetTimer` null "BillboardSystem" 1.0 true))

(event `BillboardSystem`
  (`TextRenderComponent.K2_SetText` (`self.TextRender - Score`) (`|FormatText` "{0} {1} " (`|FormatText` "Score:") (`KismetTextLibrary.Conv_IntToText` (`/Game/VirtualRealityBP/Blueprints/MotionControllerPawn.Score` (`self.As Motion Controller Pawn`)))))
  (`TextRenderComponent.K2_SetText` (`self.TextRender - Coin`) (`|FormatText` "{0} {1} " (`|FormatText` "Coin:") (`KismetTextLibrary.Conv_IntToText` (`/Game/VirtualRealityBP/Blueprints/MotionControllerPawn.Coin` (`self.As Motion Controller Pawn`))))))

(fn `UserConstructionScript`)