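; BP_Turret is a turret actor whose Fire event spawns a BP_Projectile at its Arrow component's location.
; It caches the level's BP_Train on BeginPlay and skips firing while that train is stopped.
; It also requires the player's MotionControllerPawn to have health left and be within a fixed distance of the turret.
; Nothing in this Blueprint calls Fire or aims the shot, as the spawn sets only a location.
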(event `self.ReceiveBeginPlay`
  (bind _returnvalue (`GameplayStatics.GetActorOfClass` "/Game/Blueprint/BP_Train.BP_Train_C"))
  (set `self.TrainRef` _returnvalue))

(event `Fire`
  (if (not (`/Game/Blueprint/BP_Train.IsStopped` (`self.TrainRef`)))
    (bind _asmotion_controller_pawn (cast `/Game/VirtualRealityBP/Blueprints/MotionControllerPawn` (`GameplayStatics.GetPlayerPawn` 0)))
    (if (not (<= (`/Game/VirtualRealityBP/Blueprints/MotionControllerPawn.PHealth` _asmotion_controller_pawn) 0))
      (if (not (> (`self.GetDistanceTo` (`GameplayStatics.GetPlayerPawn` 0) self) 10000.0))
        (`|SpawnActorFromClass` "/Game/Gokdeniz/YeniKod/BP_Projectile.BP_Projectile_C" (`KismetMathLibrary.MakeTransform` (`SceneComponent.K2_GetComponentLocation` (`self.Arrow`))) "Undefined" "OverrideRootScale" null null)))))

(fn `UserConstructionScript`)