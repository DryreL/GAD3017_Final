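; BP_Projectile is a projectile that lobs itself at the VR player pawn and costs it one health on hit.
; On BeginPlay it solves a toss velocity toward a lead point, predicted from the pawn's AVelocity and distance over projectile speed, with debug drawing on.
; When its sphere overlaps a BP_MotionController, it decrements pawn health, calls CrashTime on BP_Train once health runs out, then destroys itself.
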(event `self.ReceiveBeginPlay`
  (bind _returnvalue (`GameplayStatics.GetPlayerPawn` 0))
  (bind _projectilemovement (`self.ProjectileMovement`))
  (bind _returnvalue_2 (`GameplayStatics.GetActorOfClass` "/Game/Blueprint/BP_Train.BP_Train_C"))
  (set `self.BP_TrainRef` _returnvalue_2)
  (bind _tossvelocity (`GameplayStatics.BlueprintSuggestProjectileVelocity` (`self.K2_GetActorLocation`) (+ (`self.K2_GetActorLocation` _returnvalue) (* (`/Game/VirtualRealityBP/Blueprints/MotionControllerPawn.A_Velocity` (cast `/Game/VirtualRealityBP/Blueprints/MotionControllerPawn` _returnvalue :!pure true)) (/ (`self.GetDistanceTo` _returnvalue) (`self.ProjectileSpeed`)))) (`self.ProjectileSpeed`) 0.0 "DoNotTrace" 0.0 false true))
  (set `MovementComponent.Velocity` _tossvelocity _projectilemovement)
  (set `ProjectileMovementComponent.bRotationFollowsVelocity` true _projectilemovement))

(event `self.Sphere.OnComponentBeginOverlap`
  (params (OverlappedComponent :type "PrimitiveComponent Object Reference") (OtherActor :type "Actor Object Reference") (OtherComp :type "PrimitiveComponent Object Reference") (OtherBodyIndex :type Integer) (bFromSweep :type Boolean) (SweepResult :type "HitResult Structure (by ref)"))
  (cast `/Game/VirtualRealityBP/Blueprints/BP_MotionController` OtherActor)
  (bind _asmotion_controller_pawn (cast `/Game/VirtualRealityBP/Blueprints/MotionControllerPawn` (`GameplayStatics.GetPlayerPawn` 0)))
  (bind _output_get (set `/Game/VirtualRealityBP/Blueprints/MotionControllerPawn.PHealth` (- (`/Game/VirtualRealityBP/Blueprints/MotionControllerPawn.PHealth` _asmotion_controller_pawn) 1) _asmotion_controller_pawn))
  (`KismetSystemLibrary.PrintString` (`KismetStringLibrary.Concat_StrStr` (`KismetStringLibrary.Conv_IntToString` _output_get) " health left") true true (struct :`R` 1.0 :`B` 0.007701 :`A` 1.0))
  (`|ExecutionSequence`
    (:`then_0`
      (if (<= (`/Game/VirtualRealityBP/Blueprints/MotionControllerPawn.PHealth` _asmotion_controller_pawn) 0)
        (`/Game/Blueprint/BP_Train.CrashTime` (`self.BP_TrainRef`))))
    (:`then_1`
      (`self.K2_DestroyActor`))))

(fn `UserConstructionScript`)